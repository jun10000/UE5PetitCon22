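; BP_RollerCoasterRailActor is a roller coaster rail actor that builds its track mesh along an editable spline.
; Its construction script adds one spline mesh component per segment, using a configurable mesh and forward axis.
; Each piece takes position, tangent and roll from the spline points at both ends so banking follows the spline, deferring the mesh update to the last setter.
; The event graph holds no active logic.
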(fn `UserConstructionScript`
  (locals (Index :type Integer))
  (bind _spline (`self.Spline`))
  (bind _index (`local.Index`))
  (bind (_location _tangent) (`SplineComponent.GetLocationAndTangentAtSplinePoint` _spline _index "Local"))
  (bind _returnvalue (+ _index 1))
  (bind (_location_2 _tangent_2) (`SplineComponent.GetLocationAndTangentAtSplinePoint` _spline _returnvalue "Local"))
  (`/Engine/EditorBlueprintResources/StandardMacros.IsValid` (`self.SplineMesh`)
    (:`Is Valid`
      (for _index_2 (range (`SplineComponent.GetNumberOfSplineSegments` (`self.Spline`)))
        (set `local.Index` _index_2)
        (bind _returnvalue_2 (`AddComponent|NODE_AddSplineMeshComponent-0`))
        (`SceneComponent.K2_AttachToComponent` _returnvalue_2 (`self.Spline`) "None" "KeepRelative" "KeepRelative" "KeepRelative" true)
        (`StaticMeshComponent.SetStaticMesh` _returnvalue_2 (`self.SplineMesh`))
        (`SplineMeshComponent.SetStartAndEnd` _returnvalue_2 _location _tangent _location_2 _tangent_2 false)
        (`SplineMeshComponent.SetStartRollDegrees` _returnvalue_2 (`SplineComponent.GetRollAtSplinePoint` _spline _index "Local") false)
        (`SplineMeshComponent.SetEndRollDegrees` _returnvalue_2 (`SplineComponent.GetRollAtSplinePoint` _spline _returnvalue "Local") false)
        (`SplineMeshComponent.SetForwardAxis` _returnvalue_2 (`self.SplineMeshForwardAxis`) true)))))