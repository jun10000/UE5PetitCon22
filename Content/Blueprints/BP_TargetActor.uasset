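; Shootable target that awards its point value to the game instance's score and destroys itself when hit by a BP_BeamActor.
; When movement is enabled, Tick oscillates it around its starting location along a configurable direction using a time-based sine wave with offset, speed, range and reverse options.
; The construction script color-codes a dynamic M_Target material by point value and scales the actor's Y and Z axes from its diameter.
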(event `self.ReceiveBeginPlay`
  (set `self.OriginalLocation` (`self.K2_GetActorLocation`)))

(event `self.ReceiveTick`
  (params (DeltaSeconds :type "Float (single-precision)"))
  (if (`self.IsMove`)
    (`self.K2_SetActorLocation` (+ (`self.OriginalLocation`) (* (`KismetMathLibrary.Normal` (`self.MoveDirection`)) (* (`KismetMathLibrary.DegSin` (* (+ (`GameplayStatics.GetTimeSeconds`) (`self.MoveTimeOffset`)) (`self.MoveSpeedScale`) 360.0)) (/ (`self.MoveDistanceRange`) 2.0)) (`KismetMathLibrary.SelectFloat` -1.0 1.0 (`self.IsMoveReverse`)))))))

(event `self.ReceiveHit`
  (params (MyComp :type "PrimitiveComponent Object Reference") (Other :type "Actor Object Reference") (OtherComp :type "PrimitiveComponent Object Reference") (bSelfMoved :type Boolean) (HitLocation :type "Vector Structure") (HitNormal :type "Vector Structure") (NormalImpulse :type "Vector Structure") (Hit :type "HitResult Structure (by ref)"))
  (cast `/Game/Blueprints/BP_BeamActor` Other)
  (`/Game/Blueprints/BP_GameInstance.AddScore` (`/Game/Blueprints/BP_FunctionLibrary.GetMyGameInstance`) (`self.GainPoints`))
  (`self.K2_DestroyActor`))

(fn `UserConstructionScript`
  (locals (Color1 :type "LinearColor Structure" :default (struct :`R` 0.022178 :`G` 1.0 :`B` 0.332 :`A` 1.0)) (Color2 :type "LinearColor Structure" :default (struct :`R` 0.341433 :`G` 0.4729 :`B` 1.0 :`A` 1.0)))
  (bind _returnvalue (/ (`self.Diameter`) 400.0))
  (`|ExecutionSequence`
    (:`then_0`
      (switch `int` (`self.GainPoints`)
        (:`1`
          (set `local.Color1` (struct :`G` 0.666667 :`B` 1.0 :`A` 1.0))
          (set `local.Color2` (struct :`G` 0.2 :`B` 0.3 :`A` 1.0)))
        (:`2`
          (set `local.Color1` (struct :`G` 1.0 :`A` 1.0))
          (set `local.Color2` (struct :`G` 0.3 :`A` 1.0)))
        (:`3`
          (set `local.Color1` (struct :`R` 1.0 :`G` 0.833333 :`A` 1.0))
          (set `local.Color2` (struct :`R` 0.3 :`G` 0.25 :`A` 1.0)))
        (:`4`
          (set `local.Color1` (struct :`R` 1.0 :`G` 0.416667 :`A` 1.0))
          (set `local.Color2` (struct :`R` 0.3 :`G` 0.125 :`A` 1.0)))
        (:`5`
          (set `local.Color1` (struct :`R` 1.0 :`A` 1.0))
          (set `local.Color2` (struct :`R` 0.301961 :`A` 1.0)))))
    (:`then_1`
      (bind _returnvalue_2 (`KismetMaterialLibrary.CreateDynamicMaterialInstance` "/Game/Materials/M_Target.M_Target"))
      (`PrimitiveComponent.SetMaterial` (`self.StaticMesh`) 0 _returnvalue_2)
      (`MaterialInstanceDynamic.SetVectorParameterValue` _returnvalue_2 "Color1" (`local.Color1`))
      (`MaterialInstanceDynamic.SetVectorParameterValue` _returnvalue_2 "Color2" (`local.Color2`)))
    (:`then_2`
      (`self.SetActorScale3D` (`KismetMathLibrary.MakeVector` 1.0 _returnvalue _returnvalue)))))