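; Player pawn that rides a spline rail with free-look camera and fires beam actors with a sound.
; While in the Init state, Tick adds gravity, projects velocity onto the direction to a look-ahead spline point, clamps speed, then snaps to the nearest spline transform.
; The controller's rotation drives the camera relative to the pawn.
; SetRailAttachTo switches rails and saves camera world rotation, which Tick converts to local space to preserve the view.
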(event `self.ReceiveTick`
  (params (DeltaSeconds :type "Float (single-precision)"))
  (bind _returnvalue (`self.K2_GetActorLocation`))
  (bind _railattachto (`self.RailAttachTo`))
  (bind _returnvalue_2 (`KismetMathLibrary.Normal` (- (`SplineComponent.GetLocationAtDistanceAlongSpline` _railattachto (+ (`SplineComponent.GetDistanceAlongSplineAtLocation` _railattachto _returnvalue "World") (`self.NextPointDistance`)) "World") _returnvalue) 0.0))
  (switch `/Game/Blueprints/Enums/E_PlayerPawnState` (`self.CurrentState`)
    (:`NewEnumerator1`
      ;[1 1 1] 速度に重力を追加
      (bind _output_get (set `self.CurrentVelocity` (+ (`self.CurrentVelocity`) (* (`self.Gravity`) DeltaSeconds))))
      ;[1 1 1] 速度に推進力を適用
      (bind _output_get_2 (set `self.CurrentVelocity` (* (`KismetMathLibrary.FClamp` (`KismetMathLibrary.Dot_VectorVector` _output_get _returnvalue_2) (`self.SpeedMin`) (`self.SpeedMax`)) _returnvalue_2)))
      (`self.K2_SetActorTransform` (`SplineComponent.FindTransformClosestToWorldLocation` (`self.RailAttachTo`) (+ (* _output_get_2 DeltaSeconds) (`self.K2_GetActorLocation`)) "World" false))
      (if (`self.IsUpdateRailAttachTo`)
        (set `self.IsUpdateRailAttachTo` false)
        (`Controller.SetControlRotation` (`/Game/Blueprints/BP_FunctionLibrary.GetMyPlayerController`) (`KismetMathLibrary.InverseTransformRotation` (`self.GetTransform`) (`self.PrevCameraWorldRotation`))))
      (`SceneComponent.K2_SetRelativeRotation` (`self.Camera`) (`Controller.GetControlRotation` (`/Game/Blueprints/BP_FunctionLibrary.GetMyPlayerController`)) false false))))

(fn `SetCurrentState`
  (params (CurrentState :type "/Game/Blueprints/Enums/E_PlayerPawnState Enum" :default "NewEnumerator0"))
  (bind _output_get (set `self.CurrentState` CurrentState))
  (switch `/Game/Blueprints/Enums/E_PlayerPawnState` _output_get
    (:`NewEnumerator0`
      (`/Game/Blueprints/BP_FunctionLibrary.PrintRed` "BP_PlayerPawn.CurrentState -> NotInit"))))

(fn `SetRailAttachTo`
  (params (RailAttachTo :type "SplineComponent Object Reference"))
  (bind _output_get (set `self.RailAttachTo` RailAttachTo))
  (if (`KismetSystemLibrary.IsValid` _output_get)
    (`self.SetCurrentState` "NewEnumerator1")
    (set `self.IsUpdateRailAttachTo` true)
    (set `self.PrevCameraWorldRotation` (`SceneComponent.K2_GetComponentRotation` (`self.Camera`)))
    (else
      (`self.SetCurrentState` "NewEnumerator0"))))

(fn `Shoot`
  (bind _beamspawnpoint (`self.BeamSpawnPoint`))
  (bind _returnvalue (`SceneComponent.K2_GetComponentLocation` _beamspawnpoint))
  (`|SpawnActorFromClass` "/Game/Blueprints/BP_BeamActor.BP_BeamActor_C" (`KismetMathLibrary.MakeTransform` _returnvalue (`SceneComponent.K2_GetComponentRotation` _beamspawnpoint)) "Undefined" "MultiplyWithRoot" null null)
  (`GameplayStatics.PlaySoundAtLocation` "/Game/Sounds/SC_Shoot.SC_Shoot" _returnvalue (struct) 1.0 1.0 0.0 null null null null))

(fn `UserConstructionScript`)