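; Rail junction actor that joins input spline actors to a selectable output spline actor, acting as a switch for the player pawn.
; At BeginPlay it builds connecting splines to the selected output's start, draws them with instanced static meshes, and adds trigger boxes at junction ends.
; Overlapping a box attaches BP_PlayerPawn to its mapped spline.
; Changing the output moves the connectors' endpoints and rebuilds the meshes.
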(event `self.ReceiveBeginPlay`
  (`self.Init`))

(event `Event_OnChangeOutputSplineActor`
  (params (NewOutputSplineActor :type "/Game/Blueprints/BP_SplineActor Object Reference"))
  (`InstancedStaticMeshComponent.ClearInstances` (`self.InstancedStaticMesh`))
  (for _array_element (`SceneComponent.GetChildrenComponents` (`self.InstancedStaticMesh`) true)
    (bind `_asスプラインコンポーネント` (cast `SplineComponent` _array_element))
    (`|ExecutionSequence`
      (:`then_0`
        (`SplineComponent.SetLocationAtSplinePoint` `_asスプラインコンポーネント` 1 (`/Game/Blueprints/BP_FunctionLibrary.GetInfoAtSplinePoint` (`/Game/Blueprints/BP_SplineActor.Spline` NewOutputSplineActor) 0 "World") "World" true))
      (:`then_1`
        (`/Game/Blueprints/BP_FunctionLibrary.ISMComponent_AddInstancesFromSpline` (`self.InstancedStaticMesh`) `_asスプラインコンポーネント` (`self.StaticMeshLength`))))))

(fn `AddMyBoxCollisionComponent`
  (params (WorldLocation :type "Vector Structure") (TargetSpline :type "SplineComponent Object Reference (by ref)"))
  (bind _returnvalue (`AddComponent|NODE_AddBoxComponent-3`))
  (`/Game/Blueprints/BP_FunctionLibrary.InitBoxCollision` _returnvalue "Movable" WorldLocation (`KismetMathLibrary.Conv_DoubleToVector` (`self.SwitchTriggerSize`)) (`|CreateDelegate` :!event `Callback_BoxCollisionComponent_OnBeginOverlap`))
  (`BlueprintMapLibrary.Map_Add` (`self.CurrentBoxCollisionToSpline`) _returnvalue TargetSpline))

(fn `AddMySplineComponent`
  (params (StartLocation :type "Vector Structure (by ref)") (EndLocation :type "Vector Structure"))
  (returns (ReturnValue :type "SplineComponent Object Reference"))
  (bind _returnvalue (`AddComponent|NODE_AddSplineComponent-3`))
  (`/Game/Blueprints/BP_FunctionLibrary.InitSplineComponent` _returnvalue "Movable" (`|MakeArray` StartLocation EndLocation) "World")
  (return _returnvalue))

(fn `Callback_BoxCollisionComponent_OnBeginOverlap`
  (params (OverlappedComponent :type "PrimitiveComponent Object Reference") (OtherActor :type "Actor Object Reference") (OtherComp :type "PrimitiveComponent Object Reference") (OtherBodyIndex :type Integer) (bFromSweep :type Boolean) (SweepResult :type "HitResult Structure (by ref)"))
  (bind _asbp_player_pawn (cast `/Game/Blueprints/BP_PlayerPawn` OtherActor))
  (`/Game/Blueprints/BP_PlayerPawn.SetRailAttachTo` _asbp_player_pawn (`BlueprintMapLibrary.Map_Find` (`self.CurrentBoxCollisionToSpline`) OverlappedComponent))
  (return))

(fn `Init`
  (locals (CurrentInputLocation :type "Vector Structure" :default (0.0 0.0 0.0)) (CurrentOutputLocation :type "Vector Structure" :default (0.0 0.0 0.0)))
  (bind _currentinputlocation (`local.CurrentInputLocation`))
  (for _array_element (`self.InputSplineActors`)
    (`|ExecutionSequence`
      (:`then_0`
        (bind _spline (`/Game/Blueprints/BP_SplineActor.Spline` _array_element))
        (set `local.CurrentInputLocation` (`/Game/Blueprints/BP_FunctionLibrary.GetInfoAtSplinePoint` _spline (`/Game/Blueprints/BP_FunctionLibrary.GetLastSplinePointIndex` _spline) "World")))
      (:`then_1`
        (set `local.CurrentOutputLocation` (`/Game/Blueprints/BP_FunctionLibrary.GetInfoAtSplinePoint` (`/Game/Blueprints/BP_SplineActor.Spline` (`self.SelectedOutputSplineActor`)) 0 "World")))
      (:`then_2`
        (bind _returnvalue (`self.AddMySplineComponent` _currentinputlocation (`local.CurrentOutputLocation`)))
        (`self.AddMyBoxCollisionComponent` _currentinputlocation _returnvalue)
        (`/Game/Blueprints/BP_FunctionLibrary.ISMComponent_AddInstancesFromSpline` (`self.InstancedStaticMesh`) _returnvalue (`self.StaticMeshLength`)))))
  (for _array_element_2 (`self.OutputSplineActors`)
    (bind _spline_2 (`/Game/Blueprints/BP_SplineActor.Spline` _array_element_2))
    (`self.AddMyBoxCollisionComponent` (`/Game/Blueprints/BP_FunctionLibrary.GetInfoAtSplinePoint` _spline_2 0 "World") _spline_2)))

(fn `SetSelectedOutputSplineActor`
  (params (SplineActor :type "/Game/Blueprints/BP_SplineActor Object Reference (by ref)"))
  (if (`KismetArrayLibrary.Array_Contains` (`self.OutputSplineActors`) SplineActor)
    (bind _output_get (set `self.SelectedOutputSplineActor` SplineActor))
    (`self.Event_OnChangeOutputSplineActor` _output_get)
    (else
      (bind _output_get_2 (set `self.SelectedOutputSplineActor` (`|GetArrayItem` (`self.OutputSplineActors`))))
      (`self.Event_OnChangeOutputSplineActor` _output_get_2))))

(fn `SetSelectedOutputSplineIndex`
  (params (Index :type Integer))
  (bind _outputsplineactors (`self.OutputSplineActors`))
  (bind _output (`|GetArrayItem` _outputsplineactors Index))
  (if (`KismetArrayLibrary.Array_IsValidIndex` _outputsplineactors Index)
    (`/Engine/EditorBlueprintResources/StandardMacros.IsValid` _output
      (:`Is Valid`
        (if (`self.IsActorBeingDestroyed` _output)
          (`/Game/Blueprints/BP_FunctionLibrary.PrintRed` "Error: NewSelectedOutputSplineActor being destroyed")
          (else
            (`self.SetSelectedOutputSplineActor` _output))))
      (:`Is Not Valid`
        (`/Game/Blueprints/BP_FunctionLibrary.PrintRed` "Error: NewSelectedOutputSplineActor is not valid")))
    (else
      (`/Game/Blueprints/BP_FunctionLibrary.PrintRed` "Error: OutputSplineActorIndex is not valid"))))

(fn `SwitchSelectedOutputSplineActor`
  (bind _outputsplineactors (`self.OutputSplineActors`))
  (`self.SetSelectedOutputSplineActor` (`|GetArrayItem` _outputsplineactors (mod (+ (`KismetArrayLibrary.Array_Find` _outputsplineactors (`self.SelectedOutputSplineActor`)) 1) (`KismetArrayLibrary.Array_Length` _outputsplineactors)))))

(fn `UserConstructionScript`
  (locals (CurrentInputLocation :type "Vector Structure" :default (0.0 0.0 0.0)) (CurrentOutputLocation :type "Vector Structure" :default (0.0 0.0 0.0)))
  (`|ExecutionSequence`
    (:`then_0`
      ;[1 1 1] InstancedStaticMesh設定
      (`StaticMeshComponent.SetStaticMesh` (`self.InstancedStaticMesh`) (`self.StaticMesh`)))
    (:`then_1`
      ;[1 1 1] SelectedOutputSplineActor設定
      (if (and (> (`KismetArrayLibrary.Array_Length` (`self.InputSplineActors`)) 0) (> (`KismetArrayLibrary.Array_Length` (`self.OutputSplineActors`)) 0))
        (if (not (`KismetArrayLibrary.Array_Contains` (`self.OutputSplineActors`) (`self.SelectedOutputSplineActor`)))
          (set `self.SelectedOutputSplineActor` (`|GetArrayItem` (`self.OutputSplineActors`))))))))