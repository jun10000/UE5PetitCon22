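; BP_TimerComponent is a countdown timer component that fires OnTimerFinished when its time runs out.
; StartTimer stores an absolute destination date as the current time plus a duration, and Tick stops and notifies once that date passes.
; StopTimer pauses by saving the remaining time, ResumeTimer rebuilds the destination date from it, and GetTime returns the time left in either state.
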(event `self.ReceiveTick`
  (params (DeltaSeconds :type "Float (single-precision)"))
  (switch `/Game/Blueprints/Enums/E_TimerState` (`self.CurrentState`)
    (:`NewEnumerator1`
      (if (<= (`KismetMathLibrary.GetTotalMilliseconds` (- (`self.DestinationDate`) (`KismetMathLibrary.Now`))) 0.0)
        (set `self.CurrentState` "NewEnumerator0")
        (`self.OnTimerFinished`)))))

(fn `GetTime`
  (returns (ReturnValue :type "Timespan Structure"))
  (switch `/Game/Blueprints/Enums/E_TimerState` (`self.CurrentState`)
    (:`NewEnumerator0`
      (return (`self.RemainingTime`)))
    (:`NewEnumerator1`
      (return (- (`self.DestinationDate`) (`KismetMathLibrary.Now`))))))

(fn `ResumeTimer`
  (switch `/Game/Blueprints/Enums/E_TimerState` (`self.CurrentState`)
    (:`NewEnumerator0`
      (set `self.CurrentState` "NewEnumerator1")
      (set `self.DestinationDate` (+ (`KismetMathLibrary.Now`) (`self.RemainingTime`))))))

(fn `StartTimer`
  (params (Time :type "Timespan Structure"))
  (set `self.CurrentState` "NewEnumerator1")
  (set `self.DestinationDate` (+ (`KismetMathLibrary.Now`) Time)))

(fn `StopTimer`
  (set `self.CurrentState` "NewEnumerator0")
  (set `self.RemainingTime` (- (`self.DestinationDate`) (`KismetMathLibrary.Now`))))