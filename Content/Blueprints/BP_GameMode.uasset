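; BP_GameMode runs a timed, score-based round from start countdown to result screen.
; BeginPlay disables player input and plays the W_Go intro, whose OnShowGo event attaches the pawn to the nearest spline rail, starts the timer, resets the GameInstance score, shows the HUD and restores input.
; When BPTimerComponent finishes, it swaps the HUD for W_Result and switches to UI-only input with a visible cursor.
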(event `self.ReceiveBeginPlay`
  (`self.DisableInput` (`/Game/Blueprints/BP_FunctionLibrary.GetMyPlayerController`) null)
  (bind _returnvalue (`|CreateWidget` "/Game/Widgets/W_Go.W_Go_C"))
  (add `/Game/Widgets/W_Go.OnShowGo` _returnvalue (delegate `OnShowGo (W_GO)`))
  (`UserWidget.AddToViewport` _returnvalue 0)
  (`UserWidget.PlayAnimationForward` _returnvalue (`/Game/Widgets/W_Go.StartAnimation` _returnvalue) 1.0 false))

(event `OnShowGo (W_GO)`
  (bind _returnvalue (`/Game/Blueprints/BP_FunctionLibrary.GetMyPlayerController`))
  (`/Game/Blueprints/BP_PlayerPawn.SetRailAttachTo` (`/Game/Blueprints/BP_FunctionLibrary.GetMyPlayerPawn`) (`/Game/Blueprints/BP_FunctionLibrary.GetNearestSplineComponent` (`self.K2_GetActorLocation` (`/Game/Blueprints/BP_FunctionLibrary.GetMyPlayerPawn`))))
  (`/Game/Blueprints/BP_TimerComponent.StartTimer` (`self.BP_TimerComponent`) (`KismetMathLibrary.FromSeconds` (`self.GameSeconds`)))
  (`/Game/Blueprints/BP_GameInstance.ResetScore` (`/Game/Blueprints/BP_FunctionLibrary.GetMyGameInstance`))
  (bind _returnvalue_2 (`|CreateWidget` "/Game/Widgets/W_HUD.W_HUD_C"))
  (bind _output_get (set `self.HUD` _returnvalue_2))
  (`UserWidget.AddToViewport` _output_get 0)
  (`WidgetBlueprintLibrary.SetInputMode_GameOnly` _returnvalue true)
  (set `PlayerController.bShowMouseCursor` false _returnvalue)
  (`self.EnableInput` _returnvalue null))

(event `self.BP_TimerComponent.OnTimerFinished`
  (bind _returnvalue (`/Game/Blueprints/BP_FunctionLibrary.GetMyPlayerController`))
  (`Widget.RemoveFromParent` (`self.HUD`))
  (bind _returnvalue_2 (`|CreateWidget` "/Game/Widgets/W_Result.W_Result_C"))
  (`UserWidget.AddToViewport` _returnvalue_2 0)
  (`WidgetBlueprintLibrary.SetInputMode_UIOnlyEx` _returnvalue _returnvalue_2 "DoNotLock" true)
  (set `PlayerController.bShowMouseCursor` true _returnvalue))

(fn `UserConstructionScript`)