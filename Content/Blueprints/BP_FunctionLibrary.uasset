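; Blueprint function library of shared static helpers for the game.
; It offers typed getters for the player pawn, controller and game instance, plus red and green debug print shortcuts.
; Spline helpers build splines, configure spline meshes and query location, tangent and roll by point or distance, deferring updates until the last call where possible.
; Other utilities set up box collision with overlap binding and destroy tagged child components.
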(fn `DestroyChildComponentsByTag`
  (params (Parent :type "SceneComponent Object Reference") (Tag :type Name) (IsRecursive :type Boolean :default true))
  (for _array_element (`SceneComponent.GetChildrenComponents` Parent IsRecursive)
    (if (`ActorComponent.ComponentHasTag` _array_element Tag)
      (`ActorComponent.K2_DestroyComponent` _array_element))))

(fn `GetInfoAtDistanceAlongSpline`
  (params (Target :type "SplineComponent Object Reference") (Distance :type "Float (single-precision)") (CoordinateSpace :type "ESplineCoordinateSpace Enum" :default "Local"))
  (returns (Location :type "Vector Structure") (Tangent :type "Vector Structure") (Roll :type "Float (single-precision)"))
  (return (`SplineComponent.GetLocationAtDistanceAlongSpline` Target Distance CoordinateSpace) (`SplineComponent.GetTangentAtDistanceAlongSpline` Target Distance CoordinateSpace) (`SplineComponent.GetRollAtDistanceAlongSpline` Target Distance CoordinateSpace)))

(fn `GetInfoAtSplinePoint`
  (params (Target :type "SplineComponent Object Reference") (PointIndex :type Integer) (CoordinateSpace :type "ESplineCoordinateSpace Enum" :default "Local"))
  (returns (Location :type "Vector Structure") (Tangent :type "Vector Structure") (Roll :type "Float (single-precision)"))
  (bind (_location _tangent) (`SplineComponent.GetLocationAndTangentAtSplinePoint` Target PointIndex CoordinateSpace))
  (return _location _tangent (`SplineComponent.GetRollAtSplinePoint` Target PointIndex CoordinateSpace)))

(fn `GetLastSplinePointIndex`
  (params (Target :type "SplineComponent Object Reference"))
  (returns (ReturnValue :type Integer))
  (return (- (`SplineComponent.GetNumberOfSplinePoints` Target) 1)))

(fn `GetMyGameInstance`
  (returns (ReturnValue :type "/Game/Blueprints/BP_GameInstance Object Reference"))
  (return (cast `/Game/Blueprints/BP_GameInstance` (`GameplayStatics.GetGameInstance` null) :!pure true)))

(fn `GetMyPlayerController`
  (returns (ReturnValue :type "/Game/Blueprints/BP_PlayerController Object Reference"))
  (return (cast `/Game/Blueprints/BP_PlayerController` (`GameplayStatics.GetPlayerController` null) :!pure true)))

(fn `GetMyPlayerPawn`
  (returns (ReturnValue :type "/Game/Blueprints/BP_PlayerPawn Object Reference"))
  (return (cast `/Game/Blueprints/BP_PlayerPawn` (`GameplayStatics.GetPlayerPawn` null) :!pure true)))

(fn `InitBoxCollision`
  (params (Target :type "BoxComponent Object Reference") (Mobility :type "EComponentMobility Enum" :default "Movable") (WorldLocation :type "Vector Structure") (BoxExtent :type "Vector Structure") (OnBeginOverlap :type "Delegate (by ref)"))
  (`SceneComponent.SetMobility` Target Mobility)
  (`SceneComponent.K2_SetWorldLocation` Target WorldLocation false false)
  (`BoxComponent.SetBoxExtent` Target BoxExtent true)
  (add `PrimitiveComponent.OnComponentBeginOverlap` Target OnBeginOverlap))

(fn `InitSplineComponent`
  (params (Target :type "SplineComponent Object Reference") (Mobility :type "EComponentMobility Enum" :default "Movable") (Locations :type "Array of Vector Structure (by ref)") (CoordinateSpace :type "ESplineCoordinateSpace Enum" :default "Local"))
  (`SceneComponent.SetMobility` Target Mobility)
  (`SplineComponent.ClearSplinePoints` Target false)
  (for _array_element Locations
    (`SplineComponent.AddSplinePoint` Target _array_element CoordinateSpace false))
  (`SplineComponent.UpdateSpline` Target))

(fn `InitSplineMeshComponent`
  (params (Target :type "SplineMeshComponent Object Reference") (Mobility :type "EComponentMobility Enum" :default "Movable") (StaticMesh :type "StaticMesh Object Reference") (StaticMeshForwardAxis :type "ESplineMeshAxis Enum" :default "Z") (StartPosition :type "Vector Structure") (EndPosition :type "Vector Structure") (StartTangent :type "Vector Structure") (EndTangent :type "Vector Structure") (StartRoll :type "Float (single-precision)") (EndRoll :type "Float (single-precision)"))
  (`SceneComponent.SetMobility` Target Mobility)
  (`StaticMeshComponent.SetStaticMesh` Target StaticMesh)
  (`SplineMeshComponent.SetStartAndEnd` Target StartPosition StartTangent EndPosition EndTangent false)
  (`SplineMeshComponent.SetStartRollDegrees` Target StartRoll false)
  (`SplineMeshComponent.SetEndRollDegrees` Target EndRoll false)
  (`SplineMeshComponent.SetForwardAxis` Target StaticMeshForwardAxis true))

(fn `PrintGreen`
  (params (InString :type String))
  (`KismetSystemLibrary.PrintString` null InString true true (struct :`G` 1.0 :`A` 1.0) 10.0))

(fn `PrintRed`
  (params (InString :type String))
  (`KismetSystemLibrary.PrintString` null InString true true (struct :`R` 1.0 :`A` 1.0) 10.0))

(fn `SplineMeshComponent_SetEnd`
  (params (Target :type "SplineMeshComponent Object Reference") (Position :type "Vector Structure") (Tangent :type "Vector Structure") (Roll :type "Float (single-precision)") (UpdateMesh :type Boolean :default true))
  (`SplineMeshComponent.SetEndPosition` Target Position false)
  (`SplineMeshComponent.SetEndTangent` Target Tangent false)
  (`SplineMeshComponent.SetEndRollDegrees` Target Roll UpdateMesh))