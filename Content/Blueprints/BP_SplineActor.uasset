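; BP_SplineActor is an actor that repeats a chosen static mesh along its spline.
; The construction script assigns the mesh to an InstancedStaticMesh component and, if valid, divides the spline length by StaticMeshLength, rounded up, to get the instance count.
; Each instance takes the world-space transform at its distance along the spline, without spline scale.
; The event graph holds only disabled placeholder events, so there is no runtime logic.
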(fn `UserConstructionScript`
  (bind _staticmesh (`self.StaticMesh`))
  (`StaticMeshComponent.SetStaticMesh` (`self.InstancedStaticMesh`) _staticmesh)
  (`/Engine/EditorBlueprintResources/StandardMacros.IsValid` _staticmesh
    (:`Is Valid`
      (for _index (range (`KismetMathLibrary.FCeil` (/ (`SplineComponent.GetSplineLength` (`self.Spline`)) (`self.StaticMeshLength`))))
        (`InstancedStaticMeshComponent.AddInstance` (`self.InstancedStaticMesh`) (`SplineComponent.GetTransformAtDistanceAlongSpline` (`self.Spline`) (* _index (`self.StaticMeshLength`)) "World" false) true)))))